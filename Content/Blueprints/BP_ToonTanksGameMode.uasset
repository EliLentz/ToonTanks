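; Game mode Blueprint for ToonTanks that shows the match start and end screens.
; The StartGame event creates the start widget and adds it to the viewport.
; The GameOver event adds the game-over widget, then uses its WonGame flag to set a blue win message or a red loss message on the text block.
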(event EventBeginPlay)

(event EventTick
  (params (DeltaSeconds :type Float%20%28single-precision%29)))

(event EventStartGame
  (bind _returnvalue (UserInterface|CreateWidget "/Game/Widgets/WBP_StartGameWidget.WBP_StartGameWidget_C"))
  (UserInterface|Viewport|AddtoViewport _returnvalue 0))

(event EventGameOver
  (params (bWonGame :type Boolean))
  (bind _returnvalue (UserInterface|CreateWidget "/Game/Widgets/WBP_GameOverWidget.WBP_GameOverWidget_C"))
  (UserInterface|Viewport|AddtoViewport _returnvalue 0)
  (if bWonGame
    (Appearance|SetColorandOpacity (Variables|/Game/Widgets/WBP_GameOverWidget.WBP_GameOverWidget_C|GetTextBlock_0 _returnvalue) (Utilities|Struct|MakeSlateColor "(R=0.000000,G=0.411480,B=1.000000,A=1.000000)") :!class /Script/UMG.TextBlock)
    (Rendering|Components|TextRender|SetText (Variables|/Game/Widgets/WBP_GameOverWidget.WBP_GameOverWidget_C|GetTextBlock_0 _returnvalue) "Excelent!")
    (else
      (Appearance|SetColorandOpacity (Variables|/Game/Widgets/WBP_GameOverWidget.WBP_GameOverWidget_C|GetTextBlock_0 _returnvalue) (Utilities|Struct|MakeSlateColor "(R=1.000000,G=0.000000,B=0.000000,A=1.000000)") :!class /Script/UMG.TextBlock)
      (Rendering|Components|TextRender|SetText (Variables|/Game/Widgets/WBP_GameOverWidget.WBP_GameOverWidget_C|GetTextBlock_0 _returnvalue) "Game Over"))))

(fn ConstructionScript)